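; Air enemy projectile that is fired at the player and damages them on contact.
; On BeginPlay it launches its Sphere with a physics impulse toward the player's current position, without homing, and starts Niagara and sound effects.
; A short lifetime timer deactivates the effect and destroys it.
; Overlap of its Collision component with a TetrisGangCharacter's capsule destroys the projectile and calls ReceiveDamage on the character.
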(event `self.ReceiveBeginPlay`
  (`PrimitiveComponent.AddImpulse` (`self.Sphere`) (* (`KismetMathLibrary.GetDirectionUnitVector` (`self.K2_GetActorLocation`) (`self.K2_GetActorLocation` (`GameplayStatics.GetPlayerPawn` 0))) (`KismetMathLibrary.Conv_DoubleToVector` (`self.Velocity`))) "None" false)
  (`KismetSystemLibrary.K2_SetTimerDelegate` (delegate `Destroy`) 1.5)
  (`ActorComponent.Activate` (`self.NewNiagaraSystem`) false)
  (`GameplayStatics.PlaySoundAtLocation` "/Game/Sounds/2.2" (`self.K2_GetActorLocation`) (struct) 1.0 1.0 0.0 null null null null))

(event `Destroy`
  (`ActorComponent.Deactivate` (`self.NewNiagaraSystem`))
  (`self.K2_DestroyActor`))

(event `self.Collision.OnComponentBeginOverlap`
  (params (OverlappedComponent :type "PrimitiveComponent Object Reference") (OtherActor :type "Actor Object Reference") (OtherComp :type "PrimitiveComponent Object Reference") (OtherBodyIndex :type Integer) (bFromSweep :type Boolean) (SweepResult :type "HitResult Structure (by ref)"))
  (bind _astetris_gang_character (cast `TetrisGangCharacter` OtherActor))
  (cast `CapsuleComponent` OtherComp)
  (`self.K2_DestroyActor`)
  (`TetrisGangCharacter.ReceiveDamage` _astetris_gang_character))

(fn `UserConstructionScript`)