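; BP_AirEnemy is an air enemy Blueprint that continually turns to face the player.
; On BeginPlay it casts the player pawn to TetrisGangCharacter, caches it, and assigns its Character and Box components to AirMesh and BoxCollision.
; Each tick it snaps its rotation to the look-at yaw and roll toward the player, keeping pitch at zero so it stays level.
; The file contains no movement or attack logic.
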(event `self.ReceiveBeginPlay`
  (bind _astetris_gang_character (cast `TetrisGangCharacter` (`GameplayStatics.GetPlayerPawn` 0)))
  (set `self.PlayerRef` _astetris_gang_character)
  (set `self.AirMesh` (`self.Character`))
  (set `self.BoxCollision` (`self.Box`)))

(event `self.ReceiveTick`
  (params (DeltaSeconds :type "Float (single-precision)"))
  (bind (_returnvalue_roll _returnvalue_pitch _returnvalue_yaw) (`KismetMathLibrary.BreakRotator` (`KismetMathLibrary.FindLookAtRotation` (`self.K2_GetActorLocation`) (`self.K2_GetActorLocation` (`self.PlayerRef`)))))
  (`self.K2_SetActorRotation` (`KismetMathLibrary.MakeRotator` _returnvalue_roll 0.0 _returnvalue_yaw)))

(fn `UserConstructionScript`)