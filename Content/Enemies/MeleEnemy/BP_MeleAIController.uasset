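; AI controller for the melee enemy that drives it with a behavior tree and blackboard.
; On BeginPlay it starts the melee behavior tree and seeds the "Player" blackboard key with the first player pawn.
; Perception updates overwrite that key with whichever actor was reported, without checking team or sensing success.
; On possession it hands a reference to itself to the controlled MeleEnemy.
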(event `self.ReceiveBeginPlay`
  (bind _blackboardcomponent (`self.UseBlackboard` "/Game/Enemies/MeleEnemy/BB_MeleEnemy.BB_MeleEnemy"))
  (`self.RunBehaviorTree` "/Game/Enemies/MeleEnemy/BT_MeleEnemy.BT_MeleEnemy")
  (`BlackboardComponent.SetValueAsObject` _blackboardcomponent "Player" (`GameplayStatics.GetPlayerPawn` 0)))

(event `self.AIPerception.OnTargetPerceptionUpdated`
  (params (Actor :type "Actor Object Reference") (Stimulus :type "AIStimulus Structure"))
  (`BlackboardComponent.SetValueAsObject` (`AIBlueprintHelperLibrary.GetBlackboard` null) "Player" Actor))

(event `self.ReceivePossess`
  (params (PossessedPawn :type "Pawn Object Reference"))
  (bind _asmele_enemy (cast `MeleEnemy` PossessedPawn))
  (set `MeleEnemy.AICharacterController` self _asmele_enemy))

(fn `UserConstructionScript`)